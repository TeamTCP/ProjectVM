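; BP_Egg is an egg actor that spawns a VMEnemyBoss when an Alpha actor first overlaps it.
; BeginPlay caches the egg's location, and a flag makes the overlap trigger one-shot.
; A timeline's Height track moves the Box component downward from that location, and the boss spawns at the cached position when the timeline finishes.
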(event EventBeginPlay
  (Variables|Default|SetCurrentPosition (Transformation|GetActorLocation)))

(event Collision|EventActorBeginOverlap
  (params (OtherActor :type Actor%20Object%20Reference))
  (Utilities|Casting|CastToAlpha OtherActor)
  (if (not (Variables|Default|GetbFlag))
    (Variables|Default|SetbFlag true)
    (bind _height (Timeline|Timeline Play)
      (:Update
        (Transformation|SetWorldLocation (Variables|Default|GetBox) (+ (Variables|Default|GetCurrentPosition) (* _height "0.000000,0.000000,-100.000000")) false false))
      (:Finished
        (Game|SpawnActorfromClass "/Script/ProjectVM.VMEnemyBoss" (Math|Conversions|ToTransform(Vector) (Variables|Default|GetCurrentPosition)) "Undefined" "MultiplyWithRoot" 0 0)))))

(event EventTick
  (params (DeltaSeconds :type Float%20%28single-precision%29)))

(fn ConstructionScript)