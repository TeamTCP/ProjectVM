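; Base projectile that flies at a configurable speed and gravity, optionally homing on a Target actor.
; The construction script applies these settings to ProjectileMovement, and BeginPlay points the velocity at the Target if it is valid.
; A box collision hit calls the empty ProjectileImpact hook, then spawns the impact effect and sound and destroys the projectile.
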(event OnComponentHit(BoxCollision)
  (params (HitComponent :type Primitive%20Component%20Object%20Reference) (OtherActor :type Actor%20Object%20Reference) (OtherComp :type Primitive%20Component%20Object%20Reference) (NormalImpulse :type Vector :default "0, 0, 0") (Hit :type Hit%20Result%20Structure%20%28by%20ref%29))
  (bind _location (Collision|BreakHitResult Hit))
  (CallFunction|ProjectileImpact OtherActor Hit)
  (Effects|SpawnEmitteratLocation (Variables|Default|GetImpactEffect) _location)
  (Audio|PlaySoundatLocation (Variables|Default|GetImpactSound) _location "0, 0, 0" 1.0 1.0 0.0 0 0 0 0)
  (Actor|DestroyActor))

(event Custom|RotateToTarget
  (Variables|/Script/Engine.MovementComponent|SetVelocity (Variables|Default|GetProjectileMovement) (* (Math|Vector|GetUnitDirection(Vector) (Transformation|GetActorLocation) (Transformation|GetActorLocation (Variables|Default|GetTarget))) (Variables|ProjectileSettings|GetSpeed))))

(event EventBeginPlay
  (Variables|Default|GetTarget
    (:then
      (CallFunction|RotatetoTarget))
    (:else)))

(fn ConstructionScript
  (bind _projectilemovement (Variables|Default|GetProjectileMovement))
  (bind _projectilemovement_2 (Variables|Default|GetProjectileMovement))
  (Variables|/Script/Engine.ProjectileMovementComponent|SetInitialSpeed _projectilemovement (Variables|ProjectileSettings|GetSpeed))
  (Variables|/Script/Engine.ProjectileMovementComponent|SetMaxSpeed _projectilemovement (Variables|ProjectileSettings|GetSpeed))
  (Variables|/Script/Engine.ProjectileMovementComponent|SetProjectileGravityScale _projectilemovement (Variables|ProjectileSettings|GetGravity))
  (if (Variables|Default|GetIsHoming)
    (bind _target (Variables|Default|GetTarget)
      (:then
        (Variables|/Script/Engine.ProjectileMovementComponent|SetbIsHomingProjectile _projectilemovement_2 true)
        (Variables|/Script/Engine.ProjectileMovementComponent|SetHomingTargetComponent _projectilemovement_2 (Variables|/Script/Engine.Actor|GetRootComponent _target)))
      (:else))))

(fn ProjectileImpact
  (params (otherActor :type Actor%20Object%20Reference) (Hit :type Hit%20Result%20Structure)))